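; BP_Var is a practice Blueprint for working with variables and arrays, reporting values through on-screen prints.
; On BeginPlay it prints an element of the Fruits array, overwrites it with "kiwi" and prints it again.
; Disconnected leftover chains hold integer and float assignment and arithmetic exercises, plus adding a static mesh cube component with a material; none of these run.
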(event `self.ReceiveBeginPlay`
  (`KismetSystemLibrary.PrintString` (`|GetArrayItem` (`self.fruits`) 2) true true (struct :`G` 0.66 :`B` 1.0 :`A` 1.0) 3.0)
  (`KismetArrayLibrary.Array_Set` (`self.fruits`) 2 "kiwi")
  (`KismetSystemLibrary.PrintString` (`|GetArrayItem` (`self.fruits`) 2)))

(fn `UserConstructionScript`)