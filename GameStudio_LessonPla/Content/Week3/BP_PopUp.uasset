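; BP_PopUp is a trigger that toggles a pop-up widget when something begins overlapping its Box component.
; An IsVisible flag decides whether the overlap creates a WBP_PopUpParent widget on the viewport or removes the existing one.
; Showing it switches player 0 to Game and UI input with the mouse cursor, while hiding it restores game-only input and hides the cursor.
; The overlapping actor is not filtered.
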(event `self.Box.OnComponentBeginOverlap`
  (params (OverlappedComponent :type "PrimitiveComponent Object Reference") (OtherActor :type "Actor Object Reference") (OtherComp :type "PrimitiveComponent Object Reference") (OtherBodyIndex :type Integer) (bFromSweep :type Boolean) (SweepResult :type "HitResult Structure (by ref)"))
  (bind _returnvalue (`GameplayStatics.GetPlayerController` 0))
  (if (`self.isVisible`)
    (`Widget.RemoveFromParent` (stale _returnvalue_2))
    (set `self.isVisible` false)
    (`WidgetBlueprintLibrary.SetInputMode_GameOnly` _returnvalue)
    (set `PlayerController.bShowMouseCursor` false _returnvalue)
    (else
      ; if the widget is not visible we need to create it
      (bind _returnvalue_2 (`|CreateWidget` "/Game/Week3/WBP_PopUpParent.WBP_PopUpParent_C"))
      (`UserWidget.AddToViewport` _returnvalue_2 0)
      (set `self.isVisible` true)
      (`WidgetBlueprintLibrary.SetInputMode_GameAndUIEx` _returnvalue null)
      ; to get this node as an option drag out fromplayer controller
      (set `PlayerController.bShowMouseCursor` true _returnvalue)
      (if (`self.isVisible`)
        _))))

(fn `UserConstructionScript`)