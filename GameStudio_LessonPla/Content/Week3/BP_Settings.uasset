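; BP_Settings is an actor Blueprint that enables player input and uses the Y key to show the WBP_Settings widget.
; The open branch creates the widget and switches to game-and-UI input with a visible cursor; the close branch removes it and restores game-only input.
; Both branches set IsSettingsOpen to false, so if it starts false, each press creates another widget and the close branch never runs.
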(event `self.ReceiveBeginPlay`
  ; on BeginPlay enable input by creating a ref to the player controller
  (`self.EnableInput` (`GameplayStatics.GetPlayerController` 0)))

(event `Key|Y`
  (params (Key :type "Key Structure"))
  (bind _returnvalue (`GameplayStatics.GetPlayerController` 0))
  (:`Pressed`
    (if (`self.isSettingsOpen`)
      (`Widget.RemoveFromParent` (stale _returnvalue_2))
      (set `self.isSettingsOpen` false)
      (`WidgetBlueprintLibrary.SetInputMode_GameOnly` _returnvalue)
      (set `PlayerController.bShowMouseCursor` false _returnvalue)
      (else
        ; if the widget is not visible we need to create it
        (bind _returnvalue_2 (`|CreateWidget` "/Game/Week3/WBP_Settings.WBP_Settings_C"))
        (`UserWidget.AddToViewport` _returnvalue_2 0)
        (set `self.isSettingsOpen` false)
        (`WidgetBlueprintLibrary.SetInputMode_GameAndUIEx` _returnvalue null)
        ; to get this node as an option drag out fromplayer controller
        (set `PlayerController.bShowMouseCursor` true _returnvalue)))))

(fn `UserConstructionScript`)